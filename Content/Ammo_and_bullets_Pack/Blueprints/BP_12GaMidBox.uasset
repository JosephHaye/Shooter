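; Prop Blueprint for a mid-size box of 12 gauge ammo, with an adjustable cap and shells built entirely in the construction script.
; It lays out a four-row grid of shell instances on one InstancedStaticMesh, then varies their height and rotation from seeded random streams.
; A count setting removes shells, either randomly by seed or from the first index.
; Exposed variables also drive cap and ammo visibility and separate cull distances.
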(fn `UserConstructionScript`
  (bind _ammo_visible (`self.Ammo visible`))
  (`|ExecutionSequence`
    (:`then_0`
      ;[1 1 1] Cap Visible
      (`/Game/Ammo_and_bullets_Pack/Blueprints/Macroses/On-Off_Macro.On/Off Macro` (`self.StaticMeshComponent01`) (`self.Visible Cap`))
      ;[1 1 1] Cap rotation
      (`SceneComponent.K2_AddRelativeRotation` (`self.StaticMeshComponent01`) (`KismetMathLibrary.MakeRotator` 0.0 (`self.Rotation Cap`)) false false))
    (:`then_1`
      ;[1 1 1] First row
      (for _index (range 4)
        (`InstancedStaticMeshComponent.AddInstance` (`self.InstancedStaticMesh`) (`KismetMathLibrary.MakeTransform` (`KismetMathLibrary.MakeVector` 0.0 (* _index (`self.Space`))) (struct :`Pitch` -90.0)))))
    (:`then_2`
      ;[1 1 1] Second row
      (for _index_2 (range 4)
        (`InstancedStaticMeshComponent.AddInstance` (`self.InstancedStaticMesh`) (`KismetMathLibrary.MakeTransform` (`KismetMathLibrary.MakeVector` -2.1 (* _index_2 (`self.Space`))) (struct :`Pitch` -90.0)))))
    (:`then_3`
      ;[1 1 1] Third row
      (for _index_3 (range 4)
        (`InstancedStaticMeshComponent.AddInstance` (`self.InstancedStaticMesh`) (`KismetMathLibrary.MakeTransform` (`KismetMathLibrary.MakeVector` -4.2 (* _index_3 (`self.Space`))) (struct :`Pitch` -90.0)))))
    (:`then_4`
      ;[1 1 1] fourth row
      (for _index_4 (range 4)
        (`InstancedStaticMeshComponent.AddInstance` (`self.InstancedStaticMesh`) (`KismetMathLibrary.MakeTransform` (`KismetMathLibrary.MakeVector` -6.3 (* _index_4 (`self.Space`))) (struct :`Pitch` -90.0)))))
    (:`then_5`
      ;[1 1 1] Set up seed for random seed
      (set `self.Count ammo seed` (`KismetMathLibrary.MakeRandomStream` (`self.= Count ammo seed =`)))
      (set `self.Rotation ammo Seed` (`KismetMathLibrary.MakeRandomStream` (`self.= Rotation Ammo Seed =`)))
      (set `self.Height ammo Seed` (`KismetMathLibrary.MakeRandomStream` (`self.= Height ammo Seed =`))))
    (:`then_6`
      ;[1 1 1] Update Ammo Transform
      (for _index_5 (range (+ (`InstancedStaticMeshComponent.GetInstanceCount` (`self.InstancedStaticMesh`)) 1))
        (bind _outinstancetransform (`InstancedStaticMeshComponent.GetInstanceTransform` (`self.InstancedStaticMesh`) _index_5 false))
        (`InstancedStaticMeshComponent.UpdateInstanceTransform` (`self.InstancedStaticMesh`) _index_5 (`KismetMathLibrary.MakeTransform` (`KismetMathLibrary.MakeVector` (.x (.location _outinstancetransform)) (.y (.location _outinstancetransform)) (+ (.z (.location _outinstancetransform)) (`KismetMathLibrary.RandomFloatInRangeFromStream` (`self.Min ammo Height`) (`self.Max ammo Height`) (`self.Height ammo Seed`)))) (`KismetMathLibrary.MakeRotator` 0.0 -90.0 (`KismetMathLibrary.RandomFloatInRangeFromStream` (`self.Min ammo Rotation`) (`self.Max ammo Rotation`) (`self.Rotation ammo Seed`))) (1.0 1.0 1.0)) false false false)))
    (:`then_7`
      ;[1 1 1] Amount of remote ammo
      (if (`self.Use random count of ammo`)
        (for _ (range (+ (`KismetMathLibrary.FTrunc` (* (`self.Count ammo in %`) 0.16)) 1))
          (`InstancedStaticMeshComponent.RemoveInstance` (`self.InstancedStaticMesh`) (`KismetMathLibrary.RandomIntegerInRangeFromStream` 0 (`InstancedStaticMeshComponent.GetInstanceCount` (`self.InstancedStaticMesh`)) (`self.Count ammo seed`))))
        (else
          (for _ (range (`KismetMathLibrary.FTrunc` (`KismetMathLibrary.Abs` (* (`self.Count ammo in %`) 0.16))))
            (`InstancedStaticMeshComponent.RemoveInstance` (`self.InstancedStaticMesh`) 0)))))
    (:`then_8`
      ;[1 1 1] Ammo Visible
      (`SceneComponent.SetVisibility` (`self.InstancedStaticMesh`) _ammo_visible false)
      (`PrimitiveComponent.SetCastShadow` (`self.InstancedStaticMesh`) _ammo_visible))
    (:`then_9`
      ;[1 1 1] Draw Distance
      (`PrimitiveComponent.SetCullDistance` (`self.InstancedStaticMesh`) (`self.Ammo Draw Distance (0 - Infinity)`))
      (`PrimitiveComponent.SetCullDistance` (`self.StaticMeshComponent01`) (`self.Box Draw Distance (0 - Infinity)`))
      (`PrimitiveComponent.SetCullDistance` (`self.StaticMeshComponent0`) (`self.Box Draw Distance (0 - Infinity)`)))))